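; Player character Blueprint that manages the HUD, target indicators, pause menu and win/lose screens in what appears to be a tower defense game.
; BeginPlay creates the widgets, and Tick polls the player character's flags to show enemy or friendly target widgets.
; With neither target active, a destroyed generator shows defeat and a cleared last wave shows victory, each returning to the menu level after a delay.
; MenuPause pauses the game and opens a UI-only menu.
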(event EventBeginPlay
  ;[1 1 1] HUD creation
  (bind _returnvalue (UserInterface|CreateWidget "/Game/GUI/PlayerHUD.PlayerHUD_C"))
  (bind _asplayer_hud (Utilities|Casting|CastToPlayerHUD _returnvalue))
  (bind _output_get (Variables|Default|SetPlayerHUD _asplayer_hud))
  (UserInterface|Viewport|AddtoViewport _output_get 0)
  (bind _returnvalue_2 (UserInterface|CreateWidget "/Game/GUI/target_enemy2.target_enemy2_C"))
  (bind _astarget_enemy_2 (Utilities|Casting|CastTotarget_enemy2 _returnvalue_2))
  (Variables|Default|Settarget_enemy _astarget_enemy_2)
  (bind _returnvalue_3 (UserInterface|CreateWidget "/Game/GUI/target_friendly.target_friendly_C"))
  (bind _astarget_friendly (Utilities|Casting|CastTotarget_friendly _returnvalue_3))
  (Variables|Default|Settarget_friendly _astarget_friendly)
  (bind _returnvalue_4 (UserInterface|CreateWidget "/Game/GUI/defeat.defeat_C"))
  (bind _asdefeat (Utilities|Casting|CastTodefeat _returnvalue_4))
  (Variables|Default|Setdefeat _asdefeat)
  (bind _returnvalue_5 (UserInterface|CreateWidget "/Game/GUI/victory.victory_C"))
  (bind _asvictory (Utilities|Casting|CastTovictory _returnvalue_5))
  (Variables|Default|Setvictory _asvictory))

(event EventTick
  (params (DeltaSeconds :type Float%20%28single-precision%29))
  (bind _target_friendly (Variables|Default|Gettarget_friendly))
  (bind _target_enemy (Variables|Default|Gettarget_enemy))
  (bind _playerhud (Variables|Default|GetPlayerHUD))
  (bind _victory (Variables|Default|Getvictory))
  ;[1 1 1] HUD visibility
  (if (Game|IsGamePaused)
    (Widget|RemovefromParent _playerhud)
    (else
      (UserInterface|Viewport|AddtoViewport _playerhud 0)))
  (bind _asmy_character (Utilities|Casting|CastToMyCharacter (Game|GetPlayerCharacter 0)))
  (if (Variables|/Script/TowerDefense.TowerDefenseCharacter|GetIs_Monster _asmy_character)
    (UserInterface|Viewport|AddtoViewport _target_enemy 0)
    (else
      (Widget|RemovefromParent _target_enemy)
      (bind _asmy_character_2 (Utilities|Casting|CastToMyCharacter (Game|GetPlayerCharacter 0)))
      (if (Variables|/Script/TowerDefense.TowerDefenseCharacter|GetIs_Tower _asmy_character_2)
        (UserInterface|Viewport|AddtoViewport _target_friendly 0)
        (else
          (Widget|RemovefromParent _target_friendly)
          (if (Variables|/Script/TowerDefense.TowerDefenseCharacter|Getgenerator_destoyed _asmy_character)
            (UserInterface|Viewport|AddtoViewport (Variables|Default|Getdefeat) 0)
            (Utilities|FlowControl|Delay 0 3.0)
            (Widget|RemovefromParent (Variables|Default|GetPlayerHUD))
            (Game|OpenLevel(byName) 0 "menulevel" true "/Game/menu/menulevel?game=Menu -game")
            (elif (Variables|/Script/TowerDefense.TowerDefenseCharacter|Getlast_wave _asmy_character)
              (if (Variables|/Script/TowerDefense.TowerDefenseCharacter|GetnoMonster _asmy_character)
                (UserInterface|Viewport|AddtoViewport _victory 0)
                (Utilities|FlowControl|Delay 0 3.0)
                (Widget|RemovefromParent _victory)
                (Game|OpenLevel(byName) 0 "menulevel" true "/Game/menu/menulevel?game=Menu -game")))))))))

(event Input|ActionEvents|InputActionMenuPause
  (bind _returnvalue (Game|GetPlayerController 0))
  ;[1 1 1] Pause
  (:Pressed
    ;[1 1 1] HUD visibility
    (Game|SetGamePaused 0 true)
    (bind _returnvalue_2 (UserInterface|CreateWidget "/Game/menu/PauseMenu.PauseMenu_C"))
    (Input|SetInputModeUIOnly _returnvalue _returnvalue_2 false)
    (Variables|/Script/Engine.PlayerController|SetbShowMouseCursor _returnvalue true)
    (UserInterface|Viewport|AddtoViewport _returnvalue_2 0)))

(fn ConstructionScript)